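; Player character Blueprint for a shooter, extending a parent class that supplies the gun logic.
; BeginPlay runs the parent logic and plays the game music at the character's location.
; The SwitchWeapon input calls a SwitchWeapon function that delegates to SwitchGun.
; An unconnected branch in that function would save the current gun's class and ammo into MainWeapon, but never runs.
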(event `self.ReceiveBeginPlay`
  (`parent.ReceiveBeginPlay`)
  (`GameplayStatics.PlaySoundAtLocation` "/Game/AssetPacks/ShooterGame/Sounds/Music/ShooterGame_Music.ShooterGame_Music" (`self.K2_GetActorLocation`) (struct) 1.0 1.0 0.0 null null null))

(event `InputAction|SwitchWeapon`
  (params (Key :type "Key Structure"))
  (:`Pressed`
    (`self.SwitchWeapon`)))

(fn `SwitchWeapon`
  (`self.SwitchGun`))

(fn `UserConstructionScript`
  (`parent.UserConstructionScript`))